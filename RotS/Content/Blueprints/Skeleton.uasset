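; Skeleton enemy for a 2D flipbook game that fights the Samurai, with a health bar widget.
; A custom event moves it forward, and it turns around when its Box stops overlapping.
; Touching its Sphere damages both Samurai and skeleton; incoming damage, scaled up, updates the bar and at zero health shows a death flipbook before delayed destruction.
; A hitbox damage function exists but is not called here.
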(event OnComponentEndOverlap(Box)
  (params (OverlappedComponent :type Primitive%20Component%20Object%20Reference) (OtherActor :type Actor%20Object%20Reference) (OtherComp :type Primitive%20Component%20Object%20Reference) (OtherBodyIndex :type Integer))
  (CallFunction|TurnChar))

(event OnComponentBeginOverlap(Sphere)
  (params (OverlappedComponent :type Primitive%20Component%20Object%20Reference) (OtherActor :type Actor%20Object%20Reference) (OtherComp :type Primitive%20Component%20Object%20Reference) (OtherBodyIndex :type Integer) (bFromSweep :type Boolean) (SweepResult :type Hit%20Result%20Structure%20%28by%20ref%29))
  ;[1 1 1] apply damage
  (bind _assamurai (Utilities|Casting|CastToSamurai OtherActor))
  (Game|Damage|ApplyDamage self 0.7 0 0)
  (Game|Damage|ApplyDamage _assamurai 5.0 0 0))

(event Custom|MoveForward
  (Pawn|Input|AddMovementInput (Transformation|GetActorForwardVector) 1.0 false))

(event Collision|EventActorBeginOverlap
  (params (OtherActor :type Actor%20Object%20Reference)))

(event EventBeginPlay
  ;[1 1 1] set current health
  (bind _ashealthbar_skeleton (Utilities|Casting|CastToHealthbar_Skeleton (UserInterface|GetUserWidgetObject (Variables|Default|GetWidget))))
  (bind _output_get (Variables|Default|SetAs%20Healthbar%20Skeleton _ashealthbar_skeleton))
  (Variables|/Game/UI/Health-Damage_System/Healthbar_Skeleton.Healthbar_Skeleton_C|Sethealth _output_get (Variables|Default|Gethealth))
  (Variables|/Game/UI/Health-Damage_System/Healthbar_Skeleton.Healthbar_Skeleton_C|Setmaxhealth _output_get (Variables|Default|Getmaxhealth)))

(event Game|Damage|EventAnyDamage
  (params (Damage :type Float%20%28single-precision%29) (DamageType :type Damage%20Type%20Object%20Reference) (InstigatedBy :type Controller%20Object%20Reference) (DamageCauser :type Actor%20Object%20Reference))
  ;[1 1 1] deal damage, death
  (bind _output_get (Variables|Default|Sethealth (Math|Float|Truncate (- (Variables|Default|Gethealth) (* Damage 1e+02)))))
  (Default|HealthEvent (Variables|Default|GetAs%20Healthbar%20Skeleton) (Math|Integer|Clamp(Integer) _output_get 0 (Variables|Default|Getmaxhealth)))
  (if (<= (Variables|Default|Gethealth) 0)
    (Sprite|SetFlipbook (Variables|Default|GetSprite) "/Game/Assets/Enem_Chars/SkeletonDead.SkeletonDead")
    (Utilities|FlowControl|Delay 1.5)
    (Actor|DestroyActor)))

(fn ConstructionScript)

(fn TurnChar
  (Transformation|SetActorRotation (Math|Rotator|CombineRotators (Transformation|GetActorRotation) "0.000000,180.000000,0.000000")))

(fn Hitckeck
  (for _array_element (Collision|GetOverlappingActors (Variables|Default|GetHitbox) 0 :!class /Script/Engine.PrimitiveComponent)
    (if true
      (Game|Damage|ApplyDamage _array_element (Variables|Default|GetDamage) 0 0)
      (Development|PrintString "Hello"))))