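; Commander is a 2D flipbook skeleton enemy that turns around when its Box overlap ends and fights the Samurai in melee.
; Hitbox overlap starts a delayed loop that damages the Samurai unless it is blocking or dead, or the Commander is hit, while Tick drives the attack flipbook.
; Incoming damage, scaled up, reduces health and updates the healthbar widget; at zero, death flipbooks play and the actor is destroyed.
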(event OnComponentEndOverlap(Sphere)
  (params (OverlappedComponent :type Primitive%20Component%20Object%20Reference) (OtherActor :type Actor%20Object%20Reference) (OtherComp :type Primitive%20Component%20Object%20Reference) (OtherBodyIndex :type Integer))
  ;[1 1 1] apply damage
  (Utilities|Casting|CastToSamurai OtherActor)
  (Variables|Default|SetIsOverlapping false))

(event OnComponentBeginOverlap(Sphere)
  (params (OverlappedComponent :type Primitive%20Component%20Object%20Reference) (OtherActor :type Actor%20Object%20Reference) (OtherComp :type Primitive%20Component%20Object%20Reference) (OtherBodyIndex :type Integer) (bFromSweep :type Boolean) (SweepResult :type Hit%20Result%20Structure%20%28by%20ref%29))
  ;[1 1 1] apply damage
  (Utilities|Casting|CastToSamurai OtherActor)
  (Variables|Default|SetIsOverlapping true))

(event OnComponentBeginOverlap(Hitbox)
  (params (OverlappedComponent :type Primitive%20Component%20Object%20Reference) (OtherActor :type Actor%20Object%20Reference) (OtherComp :type Primitive%20Component%20Object%20Reference) (OtherBodyIndex :type Integer) (bFromSweep :type Boolean) (SweepResult :type Hit%20Result%20Structure%20%28by%20ref%29))
  ;[1 1 1] apply damage
  (Utilities|Casting|CastToSamurai OtherActor)
  (Variables|Default|SetIsoverlappingSphere true)
  (Utilities|FlowControl|DoOnce false :!label _label
    (:Completed
      (Variables|Default|Setisattack? true)
      (Utilities|FlowControl|Delay 0.5 :!label _label_2)
      (if (not (Variables|Default|GetDeadSkeleton))
        (if (Variables|Default|GetHitSkeleton)
          (goto _label_2)
          (elif (Variables|Default|GetIsoverlappingSphere)
            (bind _assamurai (Utilities|Casting|CastToSamurai (Game|GetPlayerCharacter 0)))
            (if (Variables|/Game/Blueprints/Samurai.Samurai_C|GetIs%20Dead _assamurai)
              (goto _label_2)
              (elif (Variables|/Game/Blueprints/Samurai.Samurai_C|Getbool_BLOCK_SM _assamurai)
                (goto _label_2)
                (else
                  (Game|Damage|ApplyDamage _assamurai 2e+01 0 0)
                  (goto _label_2))))
            (else
              (Variables|Default|Setisattack? false)
              (goto _label Reset))))))))

(event OnComponentEndOverlap(Hitbox)
  (params (OverlappedComponent :type Primitive%20Component%20Object%20Reference) (OtherActor :type Actor%20Object%20Reference) (OtherComp :type Primitive%20Component%20Object%20Reference) (OtherBodyIndex :type Integer))
  ;[1 1 1] apply damage
  (Utilities|Casting|CastToSamurai OtherActor)
  (Variables|Default|SetIsoverlappingSphere false))

(event OnComponentEndOverlap(Box)
  (params (OverlappedComponent :type Primitive%20Component%20Object%20Reference) (OtherActor :type Actor%20Object%20Reference) (OtherComp :type Primitive%20Component%20Object%20Reference) (OtherBodyIndex :type Integer))
  (CallFunction|TurnChar))

(event Custom|MoveForward
  (Pawn|Input|AddMovementInput (Transformation|GetActorForwardVector) 1.0 false))

(event Custom|attack
  (Sprite|SetFlipbook (Variables|Default|GetSprite) "/Game/Assets/Enem_Chars/Commander/CommanderAttack.CommanderAttack")
  (Variables|Default|Setisattack? true))

(event EventTick
  (params (DeltaSeconds :type Float%20%28single-precision%29))
  (if (Variables|Default|GetDeadSkeleton)
    (Utilities|FlowControl|DoOnce false
      (:Completed
        (Sprite|SetFlipbook (Variables|Default|GetSprite) "/Game/Assets/Enem_Chars/Commander/CommanderDead.CommanderDead")
        (Utilities|FlowControl|Delay 1.5)
        (Actor|DestroyActor)))
    (elif (Variables|Default|Getisattack?)
      (CallFunction|Attack))))

(event EventBeginPlay
  ;[1 1 1] set current health
  (bind _ashealthbar_skeleton (Utilities|Casting|CastToHealthbar_Skeleton (UserInterface|GetUserWidgetObject (Variables|Default|GetWidget))))
  (bind _output_get (Variables|Default|SetAs%20Healthbar%20Skeleton _ashealthbar_skeleton))
  (Variables|/Game/UI/Health-Damage_System/Healthbar_Skeleton.Healthbar_Skeleton_C|Sethealth _output_get (Variables|Default|Gethealth))
  (Variables|/Game/UI/Health-Damage_System/Healthbar_Skeleton.Healthbar_Skeleton_C|Setmaxhealth _output_get (Variables|Default|Getmaxhealth)))

(event Game|Damage|EventAnyDamage
  (params (Damage :type Float%20%28single-precision%29) (DamageType :type Damage%20Type%20Object%20Reference) (InstigatedBy :type Controller%20Object%20Reference) (DamageCauser :type Actor%20Object%20Reference))
  ;[1 1 1] deal damage, death
  (bind _output_get (Variables|Default|Sethealth (Math|Float|Truncate (- (Variables|Default|Gethealth) (* Damage 1e+02)))))
  (Default|HealthEvent (Variables|Default|GetAs%20Healthbar%20Skeleton) (Math|Integer|Clamp(Integer) _output_get 0 (Variables|Default|Getmaxhealth)))
  (if (<= (Variables|Default|Gethealth) 0)
    (Variables|Default|SetDeadSkeleton true)
    (Sprite|SetFlipbook (Variables|Default|GetSprite) "/Game/Assets/Enem_Chars/Skeleton/SkeletonDead.SkeletonDead")
    (Utilities|FlowControl|Delay 3.0)
    (Actor|DestroyActor)))

(fn ConstructionScript)

(fn TurnChar
  (Transformation|SetActorRotation (Math|Rotator|CombineRotators (Transformation|GetActorRotation) "0.000000,180.000000,0.000000")))