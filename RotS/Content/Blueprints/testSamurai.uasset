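; A playable 2D flipbook samurai character with horizontal movement, sprint, jump, light, heavy and sprint attacks, blocking and a pause menu.
; Input sets timed or held state booleans that lock movement, and Tick uses them to pick flipbooks and update facing.
; Light and heavy attacks damage every actor overlapping the hitbox each tick, without filtering self.
; Damage updates the controller's healthbar, and zero health spawns and possesses a new Samurai.
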(event Custom|Update_Animation
  (Sprite|SetFlipbook (Variables|Default|GetSprite) (select (AI|Components|NavMovement|IsFalling (Variables|Character|GetCharacterMovement)) "/Game/Assets/Player_Chars/Samurai/Jump/Jump_SM.Jump_SM" (select (> (Math|Vector|VectorLength (Variables|/Script/Engine.MovementComponent|GetVelocity (Variables|Character|GetCharacterMovement))) 0.0) (select (Variables|Default|Getbool_RUN_SM) "/Game/Assets/Player_Chars/Samurai/Run/Run_SM.Run_SM" "/Game/Assets/Player_Chars/Samurai/Walk/Walk_SM.Walk_SM") "/Game/Assets/Player_Chars/Samurai/Idle/Idle1.Idle1"))))

(event Custom|update_Control_Rotation
  (Utilities|IsValid (Pawn|GetController)
    (:Is%20Valid
      (Math|Float|CompareFloat (.X (Math|Vector|BreakVector (Variables|/Script/Engine.MovementComponent|GetVelocity (Variables|Character|GetCharacterMovement)))) 0.0
        (:>
          (Pawn|SetControlRotation (Pawn|GetController) (Math|Rotator|MakeRotator 0.0 0.0 0.0)))
        (:<
          (Pawn|SetControlRotation (Pawn|GetController) (Math|Rotator|MakeRotator 0.0 0.0 1.8e+02)))))))

(event Custom|Light_Attack_SM
  (Sprite|SetFlipbook (Variables|Default|GetSprite) "/Game/Assets/Player_Chars/Samurai/Attack_1/Light_Attack_SM.Light_Attack_SM"))

(event Custom|Heavy_Attack_SM
  (Sprite|SetFlipbook (Variables|Default|GetSprite) "/Game/Assets/Player_Chars/Samurai/Attack_2/Heavy_Attack_SM-Test.Heavy_Attack_SM-Test"))

(event Custom|Sprint_Attack_SM
  (Sprite|SetFlipbook (Variables|Default|GetSprite) "/Game/Assets/Player_Chars/Samurai/Attack_3/Sprint_Attack_SM.Sprint_Attack_SM"))

(event Custom|Block_SM
  (Sprite|SetFlipbook (Variables|Default|GetSprite) "/Game/Assets/Player_Chars/Samurai/Block/Block_SM.Block_SM"))

(event EventBeginPlay
  (Variables|Default|SetCurrent_Health (Variables|Default|GetMax_Health))
  (bind _ascontroller_sm (Utilities|Casting|CastToController_SM (Pawn|GetController)))
  (Default|UpdateHealthbar _ascontroller_sm (Variables|Default|GetCurrent_Health) (Variables|Default|GetMax_Health)))

(event Collision|EventActorBeginOverlap
  (params (OtherActor :type Actor%20Object%20Reference)))

(event EventTick
  (params (DeltaSeconds :type Float%20%28single-precision%29))
  (if (Variables|Default|Getbool_LA_SM)
    (if (Variables|Default|Getbool_SA_SM)
      (CallFunction|SprintAttackSM)
      (elif (Variables|Default|Getbool_HA_SM)
        (CallFunction|Hitcheck)
        (CallFunction|HeavyAttackSM)
        (else
          (CallFunction|Hitcheck)
          (CallFunction|LightAttackSM))))
    (elif (Variables|Default|Getbool_BLOCK_SM)
      (CallFunction|BlockSM)
      (else
        (CallFunction|UpdateAnimation))))
  (CallFunction|UpdateControlRotation))

(event Game|Damage|EventAnyDamage
  (params (Damage :type Float%20%28single-precision%29) (DamageType :type Damage%20Type%20Object%20Reference) (InstigatedBy :type Controller%20Object%20Reference) (DamageCauser :type Actor%20Object%20Reference))
  (Variables|Default|SetCurrent_Health (Math|Float|Clamp(Float) (- (Variables|Default|GetCurrent_Health) Damage) 0.0 (Variables|Default|GetMax_Health)))
  (bind _ascontroller_sm (Utilities|Casting|CastToController_SM (Pawn|GetController)))
  (Default|UpdateHealthbar _ascontroller_sm (Variables|Default|GetCurrent_Health) (Variables|Default|GetMax_Health))
  (Effects|SpawnEmitteratLocation 0 (Transformation|GetActorLocation))
  (if (== (Variables|Default|GetCurrent_Health) 0.0)
    (Actor|DestroyActor)
    (bind _returnvalue (Game|SpawnActorfromClass "/Game/Blueprints/Samurai.Samurai_C" (Math|Transform|MakeTransform "200.000000,80.000000,-40.000000" "0, 0, 0" "1.000000,1.000000,1.000000") "Undefined" "MultiplyWithRoot" 0 0))
    (Variables|Default|SetCurrent_Health 1e+02)
    (Pawn|Possess (Game|GetPlayerController 0) _returnvalue)))

(event Input|ActionEvents|InputActionJump_SM
  (params (Key :type Key%20Structure :default "None"))
  (:Pressed
    (if (not (Variables|Default|Getbool_CANT_MOVE))
      (Character|Jump)))
  (:Released
    (Character|StopJumping)))

(event Input|ActionEvents|InputActionLight_Attack_SM
  (params (Key :type Key%20Structure :default "None"))
  (:Pressed
    (Variables|Default|Setbool_CANT_MOVE true)
    (Variables|Default|Setbool_LA_SM true)
    (if (Variables|Default|Getbool_RUN_SM)
      (Variables|Default|Setbool_SA_SM true)
      (Utilities|FlowControl|Delay 0.5666)
      (Variables|Default|Setbool_SA_SM false)
      (else
        (Utilities|FlowControl|Delay 1.0)))
    (Variables|Default|Setbool_LA_SM false)
    (Variables|Default|Setbool_CANT_MOVE false)))

(event Input|ActionEvents|InputActionHeavy_Attack_SM
  (params (Key :type Key%20Structure :default "None"))
  (:Pressed
    (Variables|Default|Setbool_CANT_MOVE true)
    (Variables|Default|Setbool_HA_SM true)
    (Variables|Default|Setbool_LA_SM true)
    (Utilities|FlowControl|Delay 1.1)
    (Variables|Default|Setbool_CANT_MOVE false)
    (Variables|Default|Setbool_LA_SM false)
    (Variables|Default|Setbool_HA_SM false)))

(event Input|ActionEvents|InputActionSprint_SM
  (params (Key :type Key%20Structure :default "None"))
  (:Pressed
    (Variables|Default|Setbool_RUN_SM true))
  (:Released
    (Variables|Default|Setbool_RUN_SM false)))

(event Input|ActionEvents|InputActionBlock_SM
  (params (Key :type Key%20Structure :default "None"))
  (:Pressed
    (Variables|Default|Setbool_BLOCK_SM true)
    (Variables|Default|Setbool_CANT_MOVE true))
  (:Released
    (Variables|Default|Setbool_BLOCK_SM false)
    (Variables|Default|Setbool_CANT_MOVE false)))

(event Input|ActionEvents|InputActionPauseMenu
  (params (Key :type Key%20Structure :default "None"))
  (bind _returnvalue (Game|GetPlayerController 0))
  (:Pressed
    (bind _returnvalue_2 (UserInterface|CreateWidget "/Game/UI/PauseMenu.PauseMenu_C"))
    (UserInterface|Viewport|AddtoViewport _returnvalue_2 0)
    (Variables|/Script/Engine.PlayerController|SetbShowMouseCursor _returnvalue true)
    (Input|SetInputModeUIOnly _returnvalue 0 "DoNotLock" false)
    (Game|SetGamePaused true)))

(event Input|AxisEvents|InputAxisMove_Horizontal_SM
  (params (AxisValue :type Float%20%28single-precision%29))
  (if (not (Variables|Default|Getbool_CANT_MOVE))
    (if (Variables|Default|Getbool_RUN_SM)
      (Pawn|Input|AddMovementInput "0.800000,0.000000,0.000000" AxisValue false)
      (else
        (Pawn|Input|AddMovementInput "0.500000,0.000000,0.000000" AxisValue false)))))

(fn ConstructionScript)

(fn Hitcheck
  (for _array_element (Collision|GetOverlappingActors (Variables|Default|Gethitbox) 0 :!class /Script/Engine.PrimitiveComponent)
    (if true
      (Game|Damage|ApplyDamage _array_element (Variables|Default|GetDamage) 0 0)
      (Development|PrintString "Hello"))))